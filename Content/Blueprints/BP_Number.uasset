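; BP_Number is an actor that runs forward at an erratic pace, then shows a win or fail result, much like a race contestant.
; CE_SetDeltaY sets the base step and switches between running and idle; Tick then moves it along local Y by that step times a random factor.
; CE_SetResult lifts a winner, which Tick keeps spinning, or tilts a loser and stops it.
; Movement and spin are per frame, without delta-time scaling.
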(event `self.ReceiveTick`
  (params (DeltaSeconds :type "Float (single-precision)"))
  (switch `/Game/Blueprints/ENumberState` (`self.currState`)
    (:`NewEnumerator1`
      (`self.K2_AddActorWorldRotation` (`KismetMathLibrary.MakeRotator` 0.0 0.0 5.0)))
    (:`NewEnumerator3`
      (`self.K2_AddActorLocalOffset` (`KismetMathLibrary.MakeVector` 0.0 (* (`KismetMathLibrary.RandomFloatInRange` 0.1 10.0) (`self.Delta Location Y`)))))))

(event `CE_SetDeltaY`
  (params (deltaY :type "Float (double-precision)"))
  ; CE_SetDeltaY
  (bind _output_get (set `self.Delta Location Y` deltaY))
  (if (> _output_get 0.0)
    (set `self.currState` "NewEnumerator3")
    (else
      (set `self.currState` "NewEnumerator0"))))

(event `CE_SetResult`
  (params (IsWin :type Boolean))
  ; CE_SetResult
  (if IsWin
    (`self.K2_AddActorLocalOffset` (0.0 0.0 500.0))
    (set `self.currState` "NewEnumerator1")
    (else
      (`self.K2_SetActorRotation` (`KismetMathLibrary.MakeRotator` 0.0 -50.0))
      (set `self.currState` "NewEnumerator2"))))

(fn `UserConstructionScript`)